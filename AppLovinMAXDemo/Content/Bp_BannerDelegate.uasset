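; Banner ad delegate Blueprint that shows an AppLovin MAX banner on iOS and Android.
; The construction script picks the ad unit ID from the platform name.
; When the SDK initializes, it creates a bottom-center banner and sets its background color.
; When the banner-loaded event fires, it shows the banner, printing debug messages along the way.
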(event OnSdkInitializedDynamicDelegate(AppLovinMAXDelegate)
  (params (SdkConfiguration :type Sdk%20Configuration%20Structure%20%28by%20ref%29))
  (bind _adunitidentifier (Variables|Default|GetAdUnitIdentifier))
  (Development|PrintString "Loading Banner")
  (Class|AppLovinMAX|CreateBanner _adunitidentifier "BottomCenter")
  (Class|AppLovinMAX|SetBannerBackgroundColor _adunitidentifier (Math|Color|MakeColor 0 0 0)))

(event OnBannerAdLoadedDynamicDelegate(AppLovinMAXDelegate)
  (params (AdInfo :type Ad%20Info%20Structure%20%28by%20ref%29))
  (Development|PrintString "Banner Loaded")
  (Class|AppLovinMAX|ShowBanner (Variables|Default|GetAdUnitIdentifier)))

(fn ConstructionScript
  (switch string (Game|GetPlatformName)
    (:IOS
      (Variables|Default|SetAdUnitIdentifier "IOS_BANNER_AD_UNIT_ID"))
    (:Android
      (Variables|Default|SetAdUnitIdentifier "ANDROID_BANNER_AD_UNIT_ID"))))