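; Blueprint that listens to AppLovin MAX delegates to keep a rewarded ad preloaded on iOS and Android.
; The construction script picks a placeholder ad unit ID per platform, and the ad loads on SDK init and reloads after being hidden or failing to display.
; Load failures retry with capped exponential backoff, reset on a successful load.
; The reward-received event is an empty stub.
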(event OnSdkInitializedDynamicDelegate(AppLovinMAXDelegate)
  (params (SdkConfiguration :type Sdk%20Configuration%20Structure%20%28by%20ref%29))
  (Class|AppLovinMAX|LoadRewardedAd (Variables|Default|GetAdUnitIdentifier)))

(event OnRewardedAdLoadedDynamicDelegate(AppLovinMAXDelegate)
  (params (AdInfo :type Ad%20Info%20Structure%20%28by%20ref%29))
  (Variables|Default|SetRetryAttempt 0.0) ; Reset retry attempts
)

(event OnRewardedAdLoadFailedDynamicDelegate(AppLovinMAXDelegate)
  (params (AdInfo :type Ad%20Info%20Structure%20%28by%20ref%29) (AdError :type Ad%20Error%20Structure%20%28by%20ref%29))
  (bind _result (Math|Float|IncrementFloat (Variables|Default|GetRetryAttempt))
    (:%20%20
      (Utilities|FlowControl|Delay (Math|Float|Power 2.0 (Math|Float|Min(Float) _result 6.0)))
      (Class|AppLovinMAX|LoadRewardedAd (Variables|Default|GetAdUnitIdentifier)))))

(event OnRewardedAdHiddenDynamicDelegate(AppLovinMAXDelegate)
  (params (AdInfo :type Ad%20Info%20Structure%20%28by%20ref%29))
  (Class|AppLovinMAX|LoadRewardedAd (Variables|Default|GetAdUnitIdentifier)))

(event OnRewardedAdDisplayFailedDynamicDelegate(AppLovinMAXDelegate)
  (params (AdInfo :type Ad%20Info%20Structure%20%28by%20ref%29) (AdError :type Ad%20Error%20Structure%20%28by%20ref%29))
  (Class|AppLovinMAX|LoadRewardedAd (Variables|Default|GetAdUnitIdentifier)))

(event OnRewardedAdReceivedRewardDynamicDelegate(AppLovinMAXDelegate)
  (params (AdInfo :type Ad%20Info%20Structure%20%28by%20ref%29) (Reward :type Ad%20Reward%20Structure%20%28by%20ref%29)))

(fn ConstructionScript
  (switch string (Game|GetPlatformName)
    (:IOS
      (Variables|Default|SetAdUnitIdentifier "IOS_REWARDED_AD_UNIT_ID"))
    (:Android
      (Variables|Default|SetAdUnitIdentifier "ANDROID_REWARDED_AD_UNIT_ID"))))