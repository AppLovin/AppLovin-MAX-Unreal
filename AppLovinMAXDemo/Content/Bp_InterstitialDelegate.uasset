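; Blueprint delegate that keeps an AppLovin MAX interstitial ad preloaded on iOS and Android.
; The construction script selects a placeholder ad unit ID by platform.
; SDK initialization, ad hidden and display failure events trigger a load immediately.
; Load failures retry with exponential backoff capped by a maximum exponent, and a successful load resets the retry count.
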(event OnSdkInitializedDynamicDelegate(AppLovinMAXDelegate)
  (params (SdkConfiguration :type Sdk%20Configuration%20Structure%20%28by%20ref%29))
  (Class|AppLovinMAX|LoadInterstitial (Variables|Default|GetAdUnitIdentifier)))

(event OnInterstitialAdLoadedDynamicDelegate(AppLovinMAXDelegate)
  (params (AdInfo :type Ad%20Info%20Structure%20%28by%20ref%29))
  (Variables|Default|SetRetryAttempt 0.0) ; Reset retry attempts
)

(event OnInterstitialAdHiddenDynamicDelegate(AppLovinMAXDelegate)
  (params (AdInfo :type Ad%20Info%20Structure%20%28by%20ref%29))
  (Class|AppLovinMAX|LoadInterstitial (Variables|Default|GetAdUnitIdentifier)))

(event OnInterstitialAdDisplayFailedDynamicDelegate(AppLovinMAXDelegate)
  (params (AdInfo :type Ad%20Info%20Structure%20%28by%20ref%29) (AdError :type Ad%20Error%20Structure%20%28by%20ref%29))
  (Class|AppLovinMAX|LoadInterstitial (Variables|Default|GetAdUnitIdentifier)))

(event OnInterstitialAdLoadFailedDynamicDelegate(AppLovinMAXDelegate)
  (params (AdInfo :type Ad%20Info%20Structure%20%28by%20ref%29) (AdError :type Ad%20Error%20Structure%20%28by%20ref%29))
  (bind _result (Math|Float|IncrementFloat (Variables|Default|GetRetryAttempt))
    (:%20%20
      (Utilities|FlowControl|Delay (Math|Float|Power 2.0 (Math|Float|Min(Float) _result 6.0)))
      (Class|AppLovinMAX|LoadInterstitial (Variables|Default|GetAdUnitIdentifier)))))

(fn ConstructionScript
  (switch string (Game|GetPlatformName)
    (:IOS
      (Variables|Default|SetAdUnitIdentifier "IOS_INTERSTITIAL_AD_UNIT_ID"))
    (:Android
      (Variables|Default|SetAdUnitIdentifier "ANDROID_INTERSTITIAL_AD_UNIT_ID"))))