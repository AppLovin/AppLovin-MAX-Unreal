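; Blueprint that shows an AppLovin MAX MREC banner ad by handling the SDK delegate events.
; The construction script picks the ad unit ID for iOS or Android from the platform name.
; SDK initialization creates the MREC at top center, and the ad-loaded event then shows it, printing status messages along the way.
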(event OnSdkInitializedDynamicDelegate(AppLovinMAXDelegate)
  (params (SdkConfiguration :type Sdk%20Configuration%20Structure%20%28by%20ref%29))
  (Development|PrintString "Loading MREC...")
  (Class|AppLovinMAX|CreateMRec (Variables|Default|GetAdUnitIdentifier) "TopCenter"))

(event OnMRecAdLoadedDynamicDelegate(AppLovinMAXDelegate)
  (params (AdInfo :type Ad%20Info%20Structure%20%28by%20ref%29))
  (Development|PrintString "MREC loaded. Showing...")
  (Class|AppLovinMAX|ShowMRec (Variables|Default|GetAdUnitIdentifier)))

(fn ConstructionScript
  (switch string (Game|GetPlatformName)
    (:IOS
      (Variables|Default|SetAdUnitIdentifier "IOS_MREC_AD_UNIT_ID"))
    (:Android
      (Variables|Default|SetAdUnitIdentifier "ANDROID_MREC_AD_UNIT_ID"))))